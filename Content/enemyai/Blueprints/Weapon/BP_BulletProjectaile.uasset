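; BP_BulletProjectaile is a bullet projectile that deals fixed damage to whatever it hits and then destroys itself.
; On spawn, both of its sphere components are set to ignore the owning actor while moving.
; Each hit also reports an AI damage sense event, with the bullet as instigator and the player character's position as event location, regardless of who fired.
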(event `self.ReceiveBeginPlay`
  (bind _returnvalue (`self.GetOwner`))
  (`PrimitiveComponent.IgnoreActorWhenMoving` (`self.Sphere`) _returnvalue true)
  (`PrimitiveComponent.IgnoreActorWhenMoving` (`self.ProjectileSphere`) _returnvalue true))

(event `self.ReceiveHit`
  (params (MyComp :type "PrimitiveComponent Object Reference") (Other :type "Actor Object Reference") (OtherComp :type "PrimitiveComponent Object Reference") (bSelfMoved :type Boolean) (HitLocation :type "Vector Structure") (HitNormal :type "Vector Structure") (NormalImpulse :type "Vector Structure") (Hit :type "HitResult Structure (by ref)"))
  (`GameplayStatics.ApplyDamage` Other 10.0 null self)
  (`AISense_Damage.ReportDamageEvent` Other self 0.0 (`self.K2_GetActorLocation` (`GameplayStatics.GetPlayerCharacter` 0)))
  (`self.K2_DestroyActor`))

(fn `UserConstructionScript`)